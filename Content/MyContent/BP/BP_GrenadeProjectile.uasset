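; Timed grenade projectile that flashes red shortly before exploding, then destroys itself.
; BeginPlay timers start a looping FlipFlop material flash and later trigger Explode, which spawns the particle effect and applies radial damage.
; A sphere overlap feeds third-person characters to Launch, knocking them away with an upward boost and force that falls off with distance.
; The first player's camera shake also scales with distance from the blast.
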(event `self.ReceiveBeginPlay`
  (`|ExecutionSequence`
    (:`then_0`
      ;[0.04862 0 1 0.5687] Grenade / Explosion / Launch / Dégâts / Disparition / Shake & Distance
      (`KismetSystemLibrary.K2_SetTimerDelegate` (delegate `Explode`) 5.0))
    (:`then_1`
      ;[0.04862 0 1 0.5687] Grenade Flash
      (set `self.BaseMaterial` (`StaticMesh.GetMaterial` (`StaticMeshComponent.StaticMesh` (`self.Grenade`)) 0)))
    (:`then_2`
      (`KismetSystemLibrary.K2_SetTimerDelegate` (delegate `StartFlashing`) 3.0))))

(event `Explode`
  (bind _returnvalue (`self.K2_GetActorLocation`))
  ;[0.04862 0 1 0.5687] Grenade / Explosion / Launch / Dégâts / Disparition / Shake & Distance
  (`GameplayStatics.SpawnEmitterAtLocation` "/Game/MyContent/Assets/Particles/P_Grenade_Explosion_01.P_Grenade_Explosion_01" _returnvalue)
  (bind _outactors (`KismetSystemLibrary.SphereOverlapActors` _returnvalue 400.0 (`|MakeArray` "ObjectTypeQuery3" :!type "EObjectTypeQuery Enum") "/Game/ThirdPerson/Blueprints/BP_ThirdPersonCharacter.BP_ThirdPersonCharacter_C"))
  (for _array_element _outactors
    (bind _asbp_third_person_character (cast `/Game/ThirdPerson/Blueprints/BP_ThirdPersonCharacter` _array_element))
    (`self.Launch` _array_element _asbp_third_person_character))
  (`GameplayStatics.ApplyRadialDamage` :`BaseDamage` 65.0 :`Origin` _returnvalue :`DamageRadius` 475.0 :`DamageCauser` null :`InstigatedByController` null)
  (`PlayerController.ClientStartCameraShake` :`self` (`GameplayStatics.GetPlayerController` 0) :`Shake` "/Game/MyContent/BP/BP_GrenadeCameraShake.BP_GrenadeCameraShake_C" :`Scale` (`KismetMathLibrary.MapRangeClamped` (`KismetMathLibrary.Vector_Distance` (`self.K2_GetActorLocation` (`GameplayStatics.GetPlayerPawn` 0)) (`self.K2_GetActorLocation`)) 0.0 800.0 1.5 0.2))
  (`self.K2_DestroyActor`))

(event `StartFlashing`
  ;[0.04862 0 1 0.5687] Grenade Flash
  (`KismetSystemLibrary.K2_SetTimerDelegate` (delegate `ToggleFlashFast`) 0.2 true))

(event `ToggleFlashFast`
  (bind _grenade (`self.Grenade`))
  ;[0.04862 0 1 0.5687] Grenade Flash
  (`/Engine/EditorBlueprintResources/StandardMacros.FlipFlop`
    (:`A`
      (`PrimitiveComponent.SetMaterial` _grenade 0 "/Game/MyContent/Assets/Grenade/M_Grenade_FlashRed.M_Grenade_FlashRed"))
    (:`B`
      (`PrimitiveComponent.SetMaterial` _grenade 0 "/Game/MyContent/Assets/Grenade/Materials/GrenadeMat.GrenadeMat"))))

(fn `Launch`
  (params (Object :type "Object Object Reference") (self2 :type "Actor Object Reference"))
  (bind _returnvalue (`self.K2_GetActorLocation`))
  (bind _output_get (set `self.GrenadeLocation` _returnvalue))
  (bind _output_get_2 (set `self.Direction` (- (`self.K2_GetActorLocation` self2) _output_get)))
  (bind _output_get_3 (set `self.Distance` (`KismetMathLibrary.VSize` _output_get_2)))
  (bind _output_get_4 (set `self.Direction2` (`KismetMathLibrary.Normal` _output_get_2)))
  (bind _output_get_5 (set `self.LaunchVector` (* _output_get_4 (`KismetMathLibrary.MapRangeClamped` _output_get_3 0.0 400.0 1200.0 300.0))))
  (bind _asbp_third_person_character (cast `/Game/ThirdPerson/Blueprints/BP_ThirdPersonCharacter` Object))
  (`Character.LaunchCharacter` _asbp_third_person_character (`KismetMathLibrary.MakeVector` (.x _output_get_5) (.y _output_get_5) (+ (.z _output_get_5) 500.0)) true true))

(fn `UserConstructionScript`)