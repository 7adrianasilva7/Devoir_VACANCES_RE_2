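; BP_Down is a one-shot moving platform that carries the third-person character along a spline, intended as a downward ride.
; Overlapping its trigger box disables player input, attaches the character and plays a teleport sound.
; A timeline moves the actor along DownSpline by lerping distance over the spline's length, setting HasMoved to block retriggering.
; When the timeline finishes, the character is detached and input is restored.
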(event `self.TriggerBox.OnComponentBeginOverlap`
  (params (OverlappedComponent :type "PrimitiveComponent Object Reference") (OtherActor :type "Actor Object Reference") (OtherComp :type "PrimitiveComponent Object Reference") (OtherBodyIndex :type Integer) (bFromSweep :type Boolean) (SweepResult :type "HitResult Structure (by ref)"))
  (bind _returnvalue (`GameplayStatics.GetPlayerController` 0))
  (bind _downspline (`self.DownSpline`))
  ;[0.04588 0 1 0.52] Plateforme va vers le bas
  (bind _asbp_third_person_character (cast `/Game/ThirdPerson/Blueprints/BP_ThirdPersonCharacter` OtherActor))
  (set `self.PlayerRef` null)
  (if (not (`self.HasMoved`))
    (`self.DisableInput` _asbp_third_person_character _returnvalue)
    (`self.K2_AttachToActor` _asbp_third_person_character null "None" "KeepWorld" "KeepWorld" "KeepWorld" true)
    (`GameplayStatics.PlaySoundAtLocation` "/Game/MyContent/SFX/teleport.teleport" (`self.K2_GetActorLocation` _asbp_third_person_character) (struct) 1.0 1.0 0.0 null null null null)
    (bind (_direction _alpha) (`Timeline|MoveTimeline`)
      (:`Update`
        (set `self.HasMoved` true)
        (`self.K2_SetActorLocation` (`SplineComponent.GetLocationAtDistanceAlongSpline` _downspline (`KismetMathLibrary.Lerp` 0.0 (`SplineComponent.GetSplineLength` _downspline) _alpha) "World")))
      (:`Finished`
        (`self.K2_DetachFromActor` _asbp_third_person_character "KeepWorld" "KeepWorld" "KeepWorld")
        (`self.EnableInput` _asbp_third_person_character _returnvalue)))))

(fn `UserConstructionScript`)