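; BP_EnemyAI is an enemy that patrols random reachable points and chases the player at higher speed once PawnSensing sees a pawn.
; DamageBox overlap damages the player, gated by a cooldown.
; AnyDamage lowers HP; at zero it calls RemoveGlass on BP_Trophy actors, plays a death sound and destroys itself.
; Tick updates the overhead HP bar and turns it toward the camera; the seen-player flag is never cleared here.
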(event `self.DamageBox.OnComponentBeginOverlap`
  (params (OverlappedComponent :type "PrimitiveComponent Object Reference") (OtherActor :type "Actor Object Reference") (OtherComp :type "PrimitiveComponent Object Reference") (OtherBodyIndex :type Integer) (bFromSweep :type Boolean) (SweepResult :type "HitResult Structure (by ref)"))
  ;[0.04588 0 1 0.52] -15 HP au joueur si touché
  (bind _asbp_third_person_character (cast `/Game/ThirdPerson/Blueprints/BP_ThirdPersonCharacter` OtherActor))
  (if (`self.CanDamage`)
    (`GameplayStatics.ApplyDamage` _asbp_third_person_character (`self.DamageAmount`) (`self.GetController`) self)
    (set `self.CanDamage` false)
    (`KismetSystemLibrary.Delay` (`self.DamageCooldown`))
    (set `self.CanDamage` true)))

(event `self.PawnSensing.OnSeePawn`
  (params (Pawn :type "Pawn Object Reference"))
  ;[0.04588 0 1 0.52] Course le joueur s'il le voit, jusqu'à sa location
  (set `self.IsSeeingPlayer` true)
  (`self.FollowPlayer`)
  (set `CharacterMovementComponent.MaxWalkSpeed` 450.0 (`self.CharacterMovement`)))

(event `FollowPlayer`
  ;[0.04588 0 1 0.52] Course le joueur s'il le voit, jusqu'à sa location
  (if (`self.IsSeeingPlayer`)
    (`|AIMoveTo` self (0.0 0.0 0.0) (`GameplayStatics.GetPlayerCharacter` 0))))

(event `Patrol`
  ;[0.04588 0 1 0.52] Patrouille AI
  (`|AIMoveTo` self (`NavigationSystemV1.K2_GetRandomReachablePointInRadius` (`self.K2_GetActorLocation`) 1000.0 null null) null :!label _label
    (:`then`
      (`KismetSystemLibrary.Delay` 4.0)
      (set `CharacterMovementComponent.MaxWalkSpeed` 200.0 (`self.CharacterMovement`))
      (`self.Patrol`)
      (goto _label))))

(event `self.ReceiveBeginPlay`
  ;[0.04588 0 1 0.52] Patrouille AI
  (set `CharacterMovementComponent.MaxWalkSpeed` 200.0 (`self.CharacterMovement`))
  (`self.Patrol`))

(event `self.ReceiveAnyDamage`
  (params (Damage :type "Float (single-precision)") (DamageType :type "DamageType Object Reference") (InstigatedBy :type "Controller Object Reference") (DamageCauser :type "Actor Object Reference"))
  ;[0.04588 0 1 0.52] Glasse du trophée s'enlève si ennemi 0 HP
  (bind _output_get (set `self.HPCurrent` (- (`self.HPCurrent`) Damage)))
  (if (<= _output_get 0.0)
    (bind _outactors (`GameplayStatics.GetAllActorsOfClass` "/Game/MyContent/BP/BP_Trophy.BP_Trophy_C"))
    (for _array_element _outactors
      (`/Game/MyContent/BP/BP_Trophy.RemoveGlass` _array_element)
      (`GameplayStatics.PlaySoundAtLocation` "/Game/MyContent/SFX/death.death" (`self.K2_GetActorLocation`) (struct) 1.0 1.0 0.0 null null null null)
      (`self.K2_DestroyActor`))))

(event `self.ReceiveTick`
  (params (DeltaSeconds :type "Float (single-precision)"))
  (bind _hp_bar_enemy (`self.HP Bar Enemy`))
  ;[0.04588 0 1 0.52] Gestion bar percent AI
  (bind _asui_hp (cast `/Game/MyContent/UI/UI_HP` (`WidgetComponent.GetWidget` (`self.HP Bar Enemy`))))
  (`ProgressBar.SetPercent` (`/Game/MyContent/UI/UI_HP.HPBar` _asui_hp) (/ (`self.HPCurrent`) (`self.HPMax`)))
  (`SceneComponent.K2_SetWorldRotation` _hp_bar_enemy (`KismetMathLibrary.FindLookAtRotation` (`SceneComponent.K2_GetComponentLocation` _hp_bar_enemy) (`SceneComponent.K2_GetComponentLocation` (`Actor.RootComponent` (`GameplayStatics.GetPlayerCameraManager` 0)))) false false))

(fn `UserConstructionScript`)