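; BP_Trophy is the level's win pickup, a trophy with a glass collision component.
; Its RemoveGlass custom event destroys that glass collision and is not called within this Blueprint.
; When BP_ThirdPersonCharacter overlaps CollectibleCollision, the trophy destroys itself, shows the UI_Victory widget and plays applause.
; It then switches the player to UI-only input with a visible mouse cursor.
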(event `RemoveGlass`
  ;[0.04588 0 1 0.52] Custom event call : enlève la glasse / Si joueur touche trophée = gagne
  (`ActorComponent.K2_DestroyComponent` (`self.GlassCollision`)))

(event `self.CollectibleCollision.OnComponentBeginOverlap`
  (params (OverlappedComponent :type "PrimitiveComponent Object Reference") (OtherActor :type "Actor Object Reference") (OtherComp :type "PrimitiveComponent Object Reference") (OtherBodyIndex :type Integer) (bFromSweep :type Boolean) (SweepResult :type "HitResult Structure (by ref)"))
  (bind _returnvalue (`GameplayStatics.GetPlayerController` 0))
  ;[0.04588 0 1 0.52] Custom event call : enlève la glasse / Si joueur touche trophée = gagne
  (cast `/Game/ThirdPerson/Blueprints/BP_ThirdPersonCharacter` OtherActor)
  (`self.K2_DestroyActor`)
  (bind _returnvalue_2 (`|CreateWidget` "/Game/MyContent/UI/UI_Victory.UI_Victory_C"))
  (`UserWidget.AddToViewport` _returnvalue_2 0)
  (`GameplayStatics.PlaySound2D` "/Game/MyContent/SFX/applause.applause" 1.0 1.0 0.0 null null)
  (`WidgetBlueprintLibrary.SetInputMode_UIOnlyEx` _returnvalue _returnvalue_2)
  (set `PlayerController.bShowMouseCursor` true _returnvalue))

(fn `UserConstructionScript`)