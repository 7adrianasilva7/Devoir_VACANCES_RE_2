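; Damageable barrel enemy that shows a floating health bar and destroys itself when its HP runs out.
; Tick shows the HPBar only while the player is within range and HP is below full.
; AnyDamage subtracts damage from CurrentHP and updates the UI_HPenemy progress bar with the CurrentHP/MaxHP ratio.
; At zero HP it calls the OnDied dispatcher, plays a disappear sound at its location and destroys the actor.
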(event `self.ReceiveTick`
  (params (DeltaSeconds :type "Float (single-precision)"))
  ;[0.04862 0 1 0.5687] HP Bar affichage selon distance Player + ne s'affiche si full HP
  (if (and (<= (`self.GetDistanceTo` (`GameplayStatics.GetPlayerCharacter` 0)) 1500.0) (not (== (`self.CurrentHP`) (`self.MaxHP`))))
    (`SceneComponent.SetVisibility` (`self.HP_Bar`) true false)
    (else
      (`SceneComponent.SetVisibility` (`self.HP_Bar`) false false))))

(event `self.ReceiveAnyDamage`
  (params (Damage :type "Float (single-precision)") (DamageType :type "DamageType Object Reference") (InstigatedBy :type "Controller Object Reference") (DamageCauser :type "Actor Object Reference"))
  ;[0.04862 0 1 0.5687] -50 PV si dégâts
  (bind _output_get (set `self.CurrentHP` (- (`self.CurrentHP`) Damage)))
  (bind _asui_hpenemy (cast `/Game/MyContent/UI/UI_HPenemy` (`WidgetComponent.GetUserWidgetObject` (`self.GetComponentByClass` (`GameplayStatics.GetObjectClass` (`self.HP_Bar`))))))
  (`ProgressBar.SetPercent` (`/Game/MyContent/UI/UI_HPenemy.HealthBar` _asui_hpenemy) (/ _output_get (`self.MaxHP`)))
  (if (<= _output_get 0.0)
    (`self.OnDied`)
    (`GameplayStatics.PlaySoundAtLocation` "/Game/MyContent/SFX/disappear.disappear" (`self.K2_GetActorLocation`) (struct) 1.0 1.0 0.0 null null null null)
    (`self.K2_DestroyActor`)))

(fn `UserConstructionScript`)